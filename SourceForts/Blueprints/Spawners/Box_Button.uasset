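; Button actor in SourceForts that spawns a block of class BlockToSpawn when a nearby player presses F.
; Beginning overlap enables input for the instigator's player controller and shows a component; ending overlap disables input and hides it.
; F calls the Spawn2x3 event, which spawns the block at a component's world transform.
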(event `Key|F`
  (:`Pressed`
    (`self.Spawn2x3`)))

(event `Spawn2x3`
  (`|SpawnActorFromClass` (`self.BlockToSpawn`) (`SceneComponent.K2_GetComponentToWorld`)))

(event `self.ReceiveActorBeginOverlap`
  (params (OtherActor :type "Actor Object Reference"))
  (bind _returnvalue (`Controller.CastToPlayerController` (`Pawn.GetController` (`Actor.Instigator` OtherActor))))
  (`self.EnableInput` _returnvalue)
  (`SceneComponent.SetVisibility` true))

(event `self.ReceiveActorEndOverlap`
  (params (OtherActor :type "Actor Object Reference"))
  (`self.DisableInput` (stale `self.ReceiveActorBeginOverlap` _returnvalue))
  (`SceneComponent.SetVisibility` false))

(fn `UserConstructionScript`)