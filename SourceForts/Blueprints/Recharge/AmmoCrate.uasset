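; Team-colored ammo crate that, outside the build phase, lets same-team characters re-request their class choice, presumably to restock.
; Entering the trigger box enables the player's input and spawns a text component that a timeline keeps facing the pawn; leaving undoes both.
; Pressing E calls GetClientClassChoice on the pawn if a forward component line trace hits.
; The construction script sizes the trigger from UseRange and picks the team material.
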(event `self.UsableTrigger.OnComponentBeginOverlap`
  (params (OtherActor :type "Actor Object Reference") (OtherComp :type "PrimitiveComponent Object Reference") (OtherBodyIndex :type Integer) (bFromSweep :type Boolean) (SweepResult :type "EngineTypes.HitResult Structure (by ref)"))
  (bind _asu_forts_game_state (cast `/Game/SourceForts/uFortsGameState` (`GameplayStatics.GetGameState`)))
  (if (not (`/Game/SourceForts/uFortsGameState.bIsBuildPhase` _asu_forts_game_state))
    (bind _asufcharacter (cast `/Game/SourceForts/UFCharacter` OtherActor))
    (`self.CheckTeam` _asufcharacter
      (:`Match`
        (set `self.Pawn` _asufcharacter)
        (bind _asufplayer_controller (cast `/Game/SourceForts/UFPlayerController` (`Pawn.GetController` _asufcharacter)))
        (`self.EnableInput` _asufplayer_controller)
        (set `self.Presser` _asufplayer_controller)
        (bind _returnvalue (`AddComponent|Text Render Component_1` :`RelativeTransform` (`KismetMathLibrary.MakeTransform` (0.0 0.0 100.0) (struct))))
        (bind _output_get (set `self.TextRender` _returnvalue))
        (`Timeline|TextRenderLookAt` :!label _label
          (:`Update`
            (`SceneComponent.K2_SetWorldRotation` _output_get (`KismetMathLibrary.FindLookAtRotation` (`SceneComponent.K2_GetComponentLocation` _output_get) (`SceneComponent.K2_GetComponentLocation` (`self.Pawn`))) false)))))))

(event `Key|E`
  (:`Pressed`
    (bind _bislookingat (`self.TraceLookAtBox` (`self.Presser`)))
    (if _bislookingat
      (`/Game/SourceForts/UFCharacter.GetClientClassChoice` (`self.Pawn`) false))))

(event `self.UsableTrigger.OnComponentEndOverlap`
  (params (OtherActor :type "Actor Object Reference") (OtherComp :type "PrimitiveComponent Object Reference") (OtherBodyIndex :type Integer))
  (bind _asufcharacter (cast `/Game/SourceForts/UFCharacter` OtherActor))
  (bind _asufplayer_controller (cast `/Game/SourceForts/UFPlayerController` (`Pawn.GetController` _asufcharacter)))
  (`self.DisableInput` _asufplayer_controller)
  (`ActorComponent.K2_DestroyComponent` (`self.TextRender`))
  (goto _label :!via `Stop`))

(fn `TraceLookAtBox`
  (params (Presser :type "/Game/SourceForts/UFPlayerController Object Reference"))
  (returns (bIsLookingAt :type Boolean))
  (bind _returnvalue (`Controller.K2_GetPawn` Presser))
  (bind _returnvalue_2 (`self.K2_GetActorLocation` _returnvalue))
  (bind (_hitlocation _hitnormal _bonename _returnvalue_3) (`PrimitiveComponent.K2_LineTraceComponent` _returnvalue_2 (+ _returnvalue_2 (* (`self.GetActorForwardVector` _returnvalue) 1000.0))))
  (return _returnvalue_3))

(fn `UserConstructionScript`
  (bind _userange (`self.UseRange`))
  (`BoxComponent.SetBoxExtent` (`self.UsableTrigger`) _userange true)
  (`SceneComponent.K2_SetRelativeLocation` (`self.UsableTrigger`) (`KismetMathLibrary.MakeVector` 0.0 0.0 (- (.z _userange) 50.0)) false)
  (`PrimitiveComponent.SetMaterial` 0 (select `byte` (`self.TeamNum`) :`0` "/Game/SourceForts/Maps/OverloadContent/M_Dev_RedTeam.M_Dev_RedTeam" :`1` "/Game/SourceForts/Maps/OverloadContent/M_Dev_BlueTeam.M_Dev_BlueTeam" :!type "MaterialInterface Object Reference")))