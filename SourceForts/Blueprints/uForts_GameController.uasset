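; Game controller for SourceForts that switches the build phase state for build walls and gravity guns.
; Its BuildPhase function forwards the phase to an event, which calls MulticastBuildPhase.
; On authority only, that event finds every Test_Build_Wall and BP_GravGun actor and copies the BuildPhase value into each.
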(event `self.ReceiveBeginPlay`)

(event `Event BuildPhase`
  (params (BuildPhase :type Boolean :default false))
  (`self.Multicast Build Phase` BuildPhase (`self.BuildWall`)))

(event `Multicast Build Phase`
  (params (`Build Phase` :type Boolean :default false) (`Build Wall` :type "/Game/SourceForts/Blueprints/Walls/Test_Build_Wall Object Reference"))
  (`/Engine/EditorBlueprintResources/ActorMacros.Switch Has Authority`
    (:`Authority`
      (`|ExecutionSequence`
        (:`then_0`
          (bind _astest_build_wall (castclass `/Game/SourceForts/Blueprints/Walls/Test_Build_Wall` "/Game/SourceForts/Blueprints/Walls/Test_Build_Wall.Test_Build_Wall_C"))
          (bind _outactors (`GameplayStatics.GetAllActorsOfClass` _astest_build_wall))
          (for _array_element _outactors
            (set `/Game/SourceForts/Blueprints/Walls/Test_Build_Wall.Build Phase` `Build Phase` _array_element)))
        (:`then_1`
          (bind _asbp_grav_gun (castclass `/Game/SourceForts/BP_GravGun` "/Game/SourceForts/BP_GravGun.BP_GravGun_C"))
          (bind _outactors_2 (`GameplayStatics.GetAllActorsOfClass` _asbp_grav_gun))
          (for _array_element_2 _outactors_2
            (set `/Game/SourceForts/BP_GravGun.Build Phase?` `Build Phase` _array_element_2)))))))

(fn `BuildPhase`
  (params (BuildPhase :type Boolean))
  (returns (DummyOutput :type Boolean))
  (`self.Event BuildPhase` BuildPhase)
  (return false))

(fn `UserConstructionScript`)