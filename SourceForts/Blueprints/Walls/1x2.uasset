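; Physics-driven 1x2 wall block for SourceForts that shows whether it is frozen and shatters when removed.
; Each tick it sets a frozen or unfrozen material according to whether its static mesh is simulating physics.
; On EndPlay it spawns a BP_2x3_DM replacement at the mesh's relative transform, passes on linear velocity and plays a flak explosion.
; The materials and replacement class are 2x3 assets despite the 1x2 name.
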(event `self.ReceiveTick`
  (params (DeltaSeconds :type "Float (single-precision)"))
  (bind _staticmesh (`self.StaticMesh`))
  (if (`SceneComponent.IsSimulatingPhysics` _staticmesh "None")
    (`PrimitiveComponent.SetMaterial` _staticmesh 0 "/Game/SourceForts/Meshes/2x3_Unfrozen.2x3_Unfrozen")
    (else
      (`PrimitiveComponent.SetMaterial` _staticmesh 0 "/Game/SourceForts/Meshes/2x3_Frozen.2x3_Frozen"))))

(event `self.ReceiveEndPlay`
  (params (EndPlayReason :type "EngineTypes.EEndPlayReason Enum" :default "ActorDestroyed"))
  (bind _staticmesh (`self.StaticMesh`))
  (bind _returnvalue (`SceneComponent.GetRelativeTransform` _staticmesh))
  (bind _returnvalue_2 (`PrimitiveComponent.GetPhysicsLinearVelocity` _staticmesh "None"))
  (bind _returnvalue_3 (`|SpawnActorFromClass` "/Game/SourceForts/Blueprints/Walls/BP_2x3_DM.BP_2x3_DM_C" _returnvalue true))
  (`PrimitiveComponent.SetAllPhysicsLinearVelocity` _returnvalue_3 _returnvalue_2 false)
  (`GameplayStatics.SpawnEmitterAtLocation` "/Game/RestrictedAssets/Proto/UT3_Weapons/WP_FlakCannon/Effects/P_WP_Flak_Alt_Explosion.P_WP_Flak_Alt_Explosion" (`SceneComponent.K2_GetComponentLocation` _returnvalue_3) (struct) false))

(fn `UserConstructionScript`)