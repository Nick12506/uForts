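; Base fort-building block that swaps materials to show its state and can shatter when destroyed.
; Toggling picks the frozen or unfrozen material from whether the mesh is simulating physics; separate calls apply transparency or restore the unfrozen material.
; A special sentinel damage value triggers destruction, replacing the mesh with a simulated destructible component that inherits its transform and velocity and ignores pawns.
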(event `ServerToggleTexture`
  (bind _mesh (`self.Mesh`))
  (if (`SceneComponent.IsSimulatingPhysics` _mesh "None")
    (`PrimitiveComponent.SetMaterial` _mesh 0 (`self.UnfrozenMaterial`))
    (else
      (`PrimitiveComponent.SetMaterial` _mesh 0 (`self.Frozen Material`)))))

(event `Toggle_Texture`
  (`self.ServerToggleTexture`))

(event `DestroyMulticast`
  (bind _mesh (`self.Mesh`))
  (`PrimitiveComponent.SetSimulatePhysics` _mesh true)
  (bind _returnvalue (`SceneComponent.GetRelativeTransform` _mesh))
  (bind _returnvalue_2 (`PrimitiveComponent.GetPhysicsLinearVelocity` _mesh "None"))
  (bind _returnvalue_3 (`AddComponent|Destructible Component_2` :`bManualAttachment` true :`RelativeTransform` _returnvalue))
  (`PrimitiveComponent.SetSimulatePhysics` _returnvalue_3 true)
  (`DestructibleComponent.SetDestructibleMesh` _returnvalue_3 (`self.DestructibleMesh`))
  (`PrimitiveComponent.SetCollisionResponseToChannel` _returnvalue_3 "ECC_Pawn" "ECR_Ignore")
  (`PrimitiveComponent.SetPhysicsLinearVelocity` _returnvalue_3 _returnvalue_2 false "None")
  (`ActorComponent.K2_DestroyComponent` _mesh))

(event `self.ReceiveAnyDamage`
  (params (Damage :type "Float (single-precision)") (DamageType :type "DamageType Object Reference") (InstigatedBy :type "Controller Object Reference") (DamageCauser :type "Actor Object Reference"))
  (if (== Damage 99999999.0)
    (`self.DestroyMulticast`)))

(event `MakeTransparentServer`
  (`PrimitiveComponent.SetMaterial` 0 (`self.TransparentMaterial`)))

(event `MakeTransparent`
  (`self.MakeTransparentServer`))

(event `UndoTransparentServer`
  (`PrimitiveComponent.SetMaterial` 0 (`self.UnfrozenMaterial`)))

(event `UndoTransparent`
  (`self.UndoTransparentServer`))

(fn `ToggleBlock`
  (returns (DummyOutput :type Boolean))
  (`self.Toggle_Texture`)
  (return false))

(fn `TransparentBlock`
  (returns (`Dummy Output` :type Boolean))
  (`self.MakeTransparent`)
  (return false))

(fn `UnTransparentBlock`
  (returns (`Dummy Output` :type Boolean))
  (`self.UndoTransparentServer`)
  (return false))

(fn `UserConstructionScript`)