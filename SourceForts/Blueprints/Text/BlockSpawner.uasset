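; BlockSpawner animates a bobbing, spinning object; despite the name, it contains no spawning logic.
; BeginPlay caches the starting world location and a lower point directly beneath it.
; Tick ping-pongs a lerp alpha between the two points, using a Direction flag, while steadily increasing yaw.
; Both motions advance by fixed per-frame steps without delta time, so their speed depends on frame rate.
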(event `self.ReceiveTick`
  (params (DeltaSeconds :type "Float (single-precision)"))
  (if (`self.Direction`) :!label _label
    (bind _output_get (set `self.Lerp` (+ (`self.Lerp`) 0.003)))
    (if (>= _output_get 1.0)
      (set `self.Direction` false)
      (goto _label)
      (else
        _))
    (else
      (bind _output_get_2 (set `self.Lerp` (- (`self.Lerp`) 0.003)))
      (if (<= _output_get_2 0.0)
        (set `self.Direction` true)
        (goto _label)
        (else
          _))))
  (bind _output_get_3 (set `self.Rotate` (+ (`self.Rotate`) 0.5)))
  (`SceneComponent.K2_SetWorldLocationAndRotation` (`KismetMathLibrary.VLerp` (`self.Start Location`) (`self.Max Location`) (`self.Lerp`)) (`KismetMathLibrary.MakeRot` 0.0 _output_get_3)))

(event `self.ReceiveBeginPlay`
  (bind _output_get (set `self.Start Location` (`SceneComponent.K2_GetComponentLocation`)))
  (set `self.Max Location` (- _output_get (`KismetMathLibrary.MakeVector` 0.0 0.0 100.0))))

(fn `UserConstructionScript`)