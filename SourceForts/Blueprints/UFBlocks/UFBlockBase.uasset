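; Base team-owned fort block for SourceForts, with frozen, unfrozen and pawn-passable transparent material states.
; Enemy damage lowers replicated health shown through a dynamic material, while any hit above max health destroys it regardless of team.
; Death swaps the mesh for a physics destructible and has the game state recount blocks.
; Timelines dissolve it in on spawn or out before removal, and replicated flags refresh team materials and optional spinning.
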(event `CallDissolve`
  (params (Forward :type Boolean :default false))
  (`self.DissolveBlock` Forward))

(event `self.ReceiveBeginPlay`
  (`self.CallDissolve` false))

(event `ServerToggleTexture`
  (`/Engine/EditorBlueprintResources/ActorMacros.Switch Has Authority`
    (:`Authority`
      _)
    (:`Remote`
      (`KismetSystemLibrary.Delay` 0.1)))
  (`PrimitiveComponent.SetMaterial` 0 (select `bool` (`SceneComponent.IsSimulatingPhysics` (`self.Mesh`) "None") :`false` (`self.Frozen Material`) :`true` (`self.UnfrozenMaterial`)))
  (bind _returnvalue (`PrimitiveComponent.CreateDynamicMaterialInstance` 0))
  (set `self.CurrentDynamicMaterial` _returnvalue)
  (`PrimitiveComponent.SetCollisionResponseToChannel` "ECC_Pawn" "ECR_Block"))

(event `Toggle_Texture`
  (`self.ServerToggleTexture`))

(event `self.ReceiveAnyDamage`
  (params (Damage :type "Float (single-precision)") (DamageType :type "DamageType Object Reference") (InstigatedBy :type "Controller Object Reference") (DamageCauser :type "Actor Object Reference"))
  (if (`self.bIsDead`)
    _
    (elif (> Damage (`self.BlockMaxHealth`))
      (`self.DestroyMulticast`)
      (set `self.BlockState` "Dead")
      (bind _asu_forts_game_state (cast `/Game/SourceForts/uFortsGameState` (`GameplayStatics.GetGameState`)))
      (`/Game/SourceForts/uFortsGameState.CheckBlockCount` _asu_forts_game_state)
      (else
        (bind _asutplayer_controller (cast `UTPlayerController` InstigatedBy))
        (bind _asufcharacter (cast `/Game/SourceForts/UFCharacter` (`Controller.K2_GetPawn` _asutplayer_controller)))
        (if (not (== (`UTCharacter.GetTeamNum` _asufcharacter) (`self.BlockTeam`)))
          (set `self.BlockCurrentHealth` (- (`self.BlockCurrentHealth`) Damage))
          (`self.CheckIfDead`))))))

(event `DestroyMulticast`
  (bind _mesh (`self.Mesh`))
  (`PrimitiveComponent.SetSimulatePhysics` _mesh true)
  (bind _returnvalue (`SceneComponent.GetRelativeTransform` _mesh))
  (bind _returnvalue_2 (`PrimitiveComponent.GetPhysicsLinearVelocity` _mesh "None"))
  (bind _returnvalue_3 (`AddComponent|Destructible Component_2` :`bManualAttachment` true :`RelativeTransform` _returnvalue))
  (`PrimitiveComponent.SetSimulatePhysics` _returnvalue_3 true)
  (`DestructibleComponent.SetDestructibleMesh` _returnvalue_3 (`self.DestructibleMesh`))
  (`PrimitiveComponent.SetMaterial` _returnvalue_3 0 (`self.UnfrozenMaterial`))
  (`PrimitiveComponent.SetPhysicsLinearVelocity` _returnvalue_3 _returnvalue_2 false "None")
  (`ActorComponent.K2_DestroyComponent` _mesh)
  (set `self.bIsDead` true)
  (`GameplayStatics.PlaySoundAttached` (select `int` (`KismetMathLibrary.RandomIntegerInRange` 0 1) :`0` "/Game/SourceForts/Audio/Blocks/Smash1_Cue.Smash1_Cue" :`1` "/Game/SourceForts/Audio/Blocks/Smash2_Cue.Smash2_Cue" :!type "SoundBase Object Reference") (`self.Mesh`) "None" (0.0 0.0 0.0) "KeepWorldPosition")
  (`KismetSystemLibrary.Delay` 10.0)
  (`self.K2_DestroyActor`))

(event `MakeTransparentServer`
  (`/Engine/EditorBlueprintResources/ActorMacros.Switch Has Authority`
    (:`Authority`
      _)
    (:`Remote`
      (`KismetSystemLibrary.Delay` 0.1)))
  (`PrimitiveComponent.SetMaterial` 0 (`self.TransparentMaterial`))
  (`PrimitiveComponent.SetCollisionResponseToChannel` "ECC_Pawn" "ECR_Ignore"))

(event `MakeTransparent`
  (`self.MakeTransparentServer`))

(event `UndoTransparent`
  (`self.ServerToggleTexture`))

(event `DissolveBlock`
  (params (Forward :type Boolean :default false))
  (bind _mesh (`self.Mesh`))
  (bind _currentdynamicmaterial (`self.CurrentDynamicMaterial`))
  (`/Engine/EditorBlueprintResources/ActorMacros.Switch Has Authority`
    (:`Authority`
      _)
    (:`Remote`
      (`KismetSystemLibrary.Delay` 0.01)))
  (bind _particle (`self.InitializeDissolve`))
  (if Forward
    (`PrimitiveComponent.SetCollisionResponseToAllChannels` _mesh "ECR_Ignore")
    (`|ExecutionSequence`
      (:`then_0`
        (bind (_direction _dissolve) (`Timeline|DissolveOut` :!via `PlayFromStart`)
          (:`Update`
            (`MaterialInstanceDynamic.SetScalarParameterValue` (`self.CurrentDynamicMaterial`) "Dissolve" _dissolve)
            (switch `TimelineComponent.ETimelineDirection` _direction
              (:`Forward`
                (`self.K2_AddActorWorldRotation` self (`KismetMathLibrary.MakeRot` -0.2 0.0 0.0) false))))
          (:`Finished`
            (`ActorComponent.Deactivate` _particle)
            (switch `TimelineComponent.ETimelineDirection` _direction
              (:`Forward`
                (`/Engine/EditorBlueprintResources/ActorMacros.Switch Has Authority`
                  (:`Authority`
                    (`KismetSystemLibrary.Delay` 1.0)
                    (`self.K2_DestroyActor` self))))))))
      (:`then_1`
        (`KismetSystemLibrary.Delay` 0.2)
        (`PrimitiveComponent.SetSimulatePhysics` _mesh false))
      (:`then_2`
        (`KismetSystemLibrary.Delay` 0.3)
        (`ActorComponent.Activate` _particle false)))
    (else
      (bind (_direction_2 _dissolve_2 _alpha) (`Timeline|DissolveIn` :!via `PlayFromStart`)
        (:`Update`
          (`MaterialInstanceDynamic.SetScalarParameterValue` _currentdynamicmaterial "Dissolve" _dissolve_2)
          (`MaterialInstanceDynamic.SetVectorParameterValue` _currentdynamicmaterial "EdgeColor" (`KismetMathLibrary.LinearColorLerp` (select `byte` (`self.BlockTeam`) :`0` (make `Object.LinearColor` 0.0496 0.011 0.011 1.0) :`1` (make `Object.LinearColor` 0.0104 0.0238 0.0632 1.0)) (make `Object.LinearColor` 1.0 0.076 0.0 1.0) _alpha)))))))

(fn `CheckIfDead`
  (if (`KismetTextLibrary.EqualEqual_TextText` (`self.BlockState`) (`|FormatText` "Alive"))
    (if (<= (`self.BlockCurrentHealth`) 0.0)
      (`self.DestroyMulticast`)
      (set `self.BlockState` "Dead")
      (bind _asu_forts_game_state (cast `/Game/SourceForts/uFortsGameState` (`GameplayStatics.GetGameState`)))
      (`/Game/SourceForts/uFortsGameState.CheckBlockCount` _asu_forts_game_state)
      (else
        (set `self.CurrentPercentHealth` (/ (`self.BlockCurrentHealth`) (`self.BlockMaxHealth`)))))))

(fn `InitializeDissolve`
  (returns (Particle :type "ParticleSystemComponent Object Reference"))
  (bind _returnvalue (`PrimitiveComponent.CreateDynamicMaterialInstance` 0))
  (set `self.CurrentDynamicMaterial` _returnvalue)
  (`/Engine/EditorBlueprintResources/StandardMacros.IsValid` (`self.DissolveParticle`)
    (:`Is Valid`
      _)
    (:`Is Not Valid`
      (bind _returnvalue_2 (`AddComponent|Particle System Component_361`))
      (bind _output_get (set `self.DissolveParticle` _returnvalue_2))
      (`ActorComponent.Deactivate` _returnvalue_2)))
  (return _output_get))

(fn `OnRep_bIsSpinner`
  (bind _asu_forts_game_state (cast `/Game/SourceForts/uFortsGameState` (`GameplayStatics.GetGameState`)))
  (if (`/Game/SourceForts/uFortsGameState.bAllowSpinners` _asu_forts_game_state)
    (if (`self.bIsSpinner`)
      (bind _returnvalue (`AddComponent|Rotating Movement Component_0`))
      (bind _output_get (set `self.Spinner` _returnvalue))
      (set `RotatingMovementComponent.RotationRate` (`KismetMathLibrary.MakeRotator` 0.0 (`KismetMathLibrary.RandomFloatInRange` 360.0 2160.0)) _output_get)
      (else
        (`ActorComponent.K2_DestroyComponent` (`self.Spinner`))))))

(fn `OnRep_BlockTeam`
  (bind _blockteam (`self.BlockTeam`))
  (set `self.UnfrozenMaterial` (select `byte` _blockteam :`0` (`self.RedUnfrozenMaterial`) :`1` (`self.BlueUnfrozenMaterial`)))
  (set `self.Frozen Material` (select `byte` _blockteam :`0` (`self.RedFrozenMaterial`) :`1` (`self.BlueFrozenMaterial`)))
  (set `self.TransparentMaterial` (select `byte` _blockteam :`0` (`self.RedTransparentMaterial`) :`1` (`self.BlueTransparentMaterial`)))
  (bind _asu_forts_game_state (cast `/Game/SourceForts/uFortsGameState` (`GameplayStatics.GetGameState`)))
  (`/Game/SourceForts/uFortsGameState.CheckBlockCount` _asu_forts_game_state))

(fn `OnRep_CurrentDynamicMaterial`
  (`MaterialInstanceDynamic.SetScalarParameterValue` (`self.CurrentDynamicMaterial`) "Alpha" (`self.CurrentPercentHealth`)))

(fn `OnRep_CurrentPercentHealth`
  (`MaterialInstanceDynamic.SetScalarParameterValue` (`self.CurrentDynamicMaterial`) "Alpha" (`self.CurrentPercentHealth`)))

(fn `ToggleBlock`
  (returns (DummyOutput :type Boolean))
  (`self.Toggle_Texture`)
  (return false))

(fn `TransparentBlock`
  (returns (`Dummy Output` :type Boolean))
  (`self.MakeTransparent`)
  (return false))

(fn `UnTransparentBlock`
  (returns (`Dummy Output` :type Boolean))
  (`self.UndoTransparent`)
  (return false))

(fn `UserConstructionScript`
  (bind _blockteam (`self.BlockTeam`))
  (set `self.BlockCurrentHealth` (`self.BlockMaxHealth`))
  (set `self.UnfrozenMaterial` (select `byte` _blockteam :`0` (`self.RedUnfrozenMaterial`) :`1` (`self.BlueUnfrozenMaterial`)))
  (set `self.Frozen Material` (select `byte` _blockteam :`0` (`self.RedFrozenMaterial`) :`1` (`self.BlueFrozenMaterial`)))
  (set `self.TransparentMaterial` (select `byte` _blockteam :`0` (`self.RedTransparentMaterial`) :`1` (`self.BlueTransparentMaterial`)))
  (`self.ServerToggleTexture`)
  (`/Engine/EditorBlueprintResources/ActorMacros.Switch Has Authority`
    (:`Remote`
      (`MaterialInstanceDynamic.SetScalarParameterValue` (`self.CurrentDynamicMaterial`) "Dissolve" 0.06))))