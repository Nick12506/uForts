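; BP_GrenadeProj is the grenade launcher's projectile, which detonates on a timed fuse and shows its shooter's team through its trail.
; On BeginPlay it starts a named timer for Detonate, which calls Explode at the grenade's current location with a zero hit normal.
; If the Instigator is a UFCharacter, its team number selects the color applied to both Trail color parameters.
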(event `self.ReceiveBeginPlay`
  (bind _trail (`self.Trail`))
  (`KismetSystemLibrary.K2_SetTimer` null "Detonate" 5.0)
  (bind _asufcharacter (cast `/Game/SourceForts/UFCharacter` (`self.Instigator`)))
  (bind _returnvalue (select `byte` (`UTCharacter.GetTeamNum` _asufcharacter) :`0` (struct :`R` 10.0 :`B` 0.050206 :`A` 1.0) :`1` (struct :`R` 0.029875 :`B` 10.0 :`A` 1.0) :!type "Object.LinearColor Structure"))
  (`ParticleSystemComponent.SetColorParameter` _trail "Color1" _returnvalue)
  (`ParticleSystemComponent.SetColorParameter` _trail "Color2" _returnvalue))

(fn `Detonate`
  (`self.Explode` (`self.K2_GetActorLocation`) (`KismetMathLibrary.MakeVector` 0.0)))

(fn `UserConstructionScript`)