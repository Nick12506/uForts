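; BP_SpeedToken is a spinning pickup for the Speed mode that rewards the player by pushing their BeginTime later by TimeReward.
; On capsule overlap, it records itself in the character's CollectedTokens to block repeat pickups, then updates the PlayerState found through the controller.
; Outside dedicated servers, only the first local player's pickup plays sound and particles, hides the token and notifies the HUD's speed widget.
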(event `self.ReceiveTick`
  (params (DeltaSeconds :type "Float (single-precision)"))
  (`SceneComponent.K2_AddLocalRotation` (`self.SM_Logo`) (struct :`Yaw` 2.0) false))

(event `self.Capsule1.OnComponentBeginOverlap`
  (params (OtherActor :type "Actor Object Reference") (OtherComp :type "PrimitiveComponent Object Reference") (OtherBodyIndex :type Integer) (bFromSweep :type Boolean) (SweepResult :type "EngineTypes.HitResult Structure (by ref)"))
  (bind _returnvalue (`self.K2_GetActorLocation`))
  (bind _asbp_speed_character (cast `/Game/Speed/Blueprints/BP_SpeedCharacter` OtherActor))
  (bind _collectedtokens (`/Game/Speed/Blueprints/BP_SpeedCharacter.CollectedTokens` _asbp_speed_character))
  (if (not (`KismetArrayLibrary.Array_Contains` _collectedtokens self))
    (`KismetArrayLibrary.Array_Add` _collectedtokens self)
    (bind _asbp_speed_player_state (cast `/Game/Speed/Blueprints/BP_SpeedPlayerState` (`Controller.PlayerState` (`Pawn.GetController` _asbp_speed_character))))
    (set `/Game/Speed/Blueprints/BP_SpeedPlayerState.BeginTime` (+ (`/Game/Speed/Blueprints/BP_SpeedPlayerState.BeginTime` _asbp_speed_player_state) (`self.TimeReward`)) _asbp_speed_player_state)
    (if (not (`KismetSystemLibrary.IsDedicatedServer`))
      (bind _asbp_speed_player_state_2 (cast `/Game/Speed/Blueprints/BP_SpeedPlayerState` (`Controller.PlayerState` (`GameplayStatics.GetPlayerController` 0))))
      (if (== _asbp_speed_player_state _asbp_speed_player_state_2)
        (`GameplayStatics.PlaySoundAtLocation` "/Game/RestrictedAssets/Pickups/Armor/Assets/A_Pickups_Shieldbelt_Activate_Cue.A_Pickups_Shieldbelt_Activate_Cue" _returnvalue 1.0 1.5)
        (bind _returnvalue_2 (`GameplayStatics.SpawnEmitterAtLocation` "/Game/RestrictedAssets/Tutorials/PS_TokenPickUp.PS_TokenPickUp" _returnvalue))
        (`SceneComponent.DetachFromParent` _returnvalue_2 true)
        (`self.SetActorHiddenInGame` true)
        (bind _asbp_speed_hud (cast `/Game/Speed/Blueprints/BP_SpeedHUD` (`PlayerController.GetHUD` (`GameplayStatics.GetPlayerController` 0))))
        (bind _aswb_speed_widget (cast `/Game/Speed/UMG/WB_SpeedWidget` (`/Game/Speed/Blueprints/BP_SpeedHUD.SpeedWidget` _asbp_speed_hud)))
        (`/Game/Speed/UMG/WB_SpeedWidget.PickupToken` _aswb_speed_widget (`self.TimeReward`))))))

(fn `UserConstructionScript`)