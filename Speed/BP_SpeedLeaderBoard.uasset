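; World leaderboard display actor that shows a WB_LeaderBoard widget inside a resizable mesh frame.
; The construction script positions corners, scales edges and background from two frame corner vectors, adds a dynamic icon material, and fits the widget to the frame.
; Outside dedicated servers, BeginPlay starts a retry timer until the widget exists, then passes it the starting entry and entry count once, working around setup timing issues.
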(event `self.ReceiveBeginPlay`
  (`self.SetupText`)
  (if (not (`KismetSystemLibrary.IsDedicatedServer`))
    (`KismetSystemLibrary.K2_SetTimerDelegate` (delegate `InitLoop`) 0.2)))

(event `InitLoop`
  (bind _returnvalue (`WidgetComponent.GetUserWidgetObject`))
  ;[1 1 1] seems to be some timing issues. loop until we are setup
  (if (`KismetSystemLibrary.IsValid` _returnvalue)
    (if (not (`self.bsetup`))
      (bind _aswb_leader_board (cast `/Game/Speed/UMG/WB_LeaderBoard` _returnvalue))
      (`/Game/Speed/UMG/WB_LeaderBoard.OnSetStartEntry` _aswb_leader_board (`self.StartingEntry`) (`self.NumEntries`))
      (set `self.bsetup` true))
    (else
      (`KismetSystemLibrary.K2_SetTimerDelegate` (delegate `InitLoop`) 0.2))))

(fn `SetupFrame`
  (bind _returnvalue (+ (`KismetMathLibrary.Abs` (.z (`self.Frame_TopLeft`))) (`KismetMathLibrary.Abs` (.z (`self.Frame_BottomRight`)))))
  (bind _returnvalue_2 (+ (`KismetMathLibrary.Abs` (.y (`self.Frame_TopLeft`))) (`KismetMathLibrary.Abs` (.y (`self.Frame_BottomRight`)))))
  (`SceneComponent.K2_SetRelativeLocation` (`self.SM_Corner_TopLeft`) (`self.Frame_TopLeft`) false)
  (`SceneComponent.K2_SetRelativeLocation` (`self.SM_Corner_BottomRight`) (`self.Frame_BottomRight`) false)
  (`SceneComponent.K2_SetRelativeLocation` (`self.SM_Corner_BottomLeft`) (`KismetMathLibrary.MakeVector` 0.0 (.y (`self.Frame_TopLeft`)) (.z (`self.Frame_BottomRight`))) false)
  (`SceneComponent.K2_SetRelativeLocation` (`self.SM_Corner_TopRight`) (`KismetMathLibrary.MakeVector` 0.0 (.y (`self.Frame_BottomRight`)) (.z (`self.Frame_TopLeft`))) false)
  (`SceneComponent.SetRelativeScale3D` (`self.SM_Straight_Right`) (`KismetMathLibrary.MakeVector` 1.0 (/ _returnvalue 50.0) 1.0))
  (`SceneComponent.SetRelativeScale3D` (`self.SM_Straight_Left`) (`KismetMathLibrary.MakeVector` 1.0 (/ _returnvalue 50.0) 1.0))
  (`SceneComponent.SetRelativeScale3D` (`self.SM_Straight_Top`) (`KismetMathLibrary.MakeVector` 1.0 (/ _returnvalue_2 50.0) 1.0))
  (`SceneComponent.SetRelativeScale3D` (`self.SM_Straight_Bottom`) (`KismetMathLibrary.MakeVector` 1.0 (/ _returnvalue_2 50.0) 1.0))
  (`SceneComponent.SetRelativeScale3D` (`self.SM_BG`) (`KismetMathLibrary.MakeVector` (/ (+ _returnvalue_2 20.0) 50.0) (/ (+ _returnvalue 20.0) 50.0) 0.5))
  (`SceneComponent.K2_SetRelativeLocation` (`self.SM_Icon`) (`KismetMathLibrary.MakeVector` 25.0 (+ (.y (`self.Frame_BottomRight`)) 20.0) (+ (.z (`self.Frame_TopLeft`)) 20.0)) false)
  (bind _returnvalue_3 (`PrimitiveComponent.CreateDynamicMaterialInstance` (`self.SM_Icon`) 0 null))
  (set `self.MID_Icon` _returnvalue_3))

(fn `SetupText`
  (bind _frame_topleft (`self.Frame_TopLeft`))
  (bind _frame_bottomright (`self.Frame_BottomRight`))
  (bind _widget_text_a (`self.Widget_Text_A`))
  (bind _y (.y _frame_topleft))
  (bind _z (.z _frame_topleft))
  (bind _y_2 (.y _frame_bottomright))
  (bind _z_2 (.z _frame_bottomright))
  (bind _returnvalue (`KismetMathLibrary.FClamp` (.y _frame_topleft) _y_2 _y))
  (bind _returnvalue_2 (`KismetMathLibrary.FClamp` (.z _frame_topleft) _z_2 _z))
  (cast `/Game/Speed/UMG/WB_LeaderBoard` (`WidgetComponent.GetUserWidgetObject` (`self.Widget_Text_A`)))
  (`SceneComponent.K2_SetRelativeLocation` _widget_text_a (`KismetMathLibrary.MakeVector` 2.0 _returnvalue _returnvalue_2) false)
  (`WidgetComponent.SetDrawSize` _widget_text_a (`KismetMathLibrary.MakeVector2D` (- _returnvalue (`KismetMathLibrary.FClamp` (.y _frame_bottomright) _y_2 _y)) (- _returnvalue_2 (`KismetMathLibrary.FClamp` (.z _frame_bottomright) _z_2 _z))))
  (return))

(fn `UserConstructionScript`
  (`self.SetupFrame`)
  (`self.SetupText`))