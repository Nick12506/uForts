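; Shootable per-player switch for the Speed mode that triggers its linked TriggerMover actors when damaged by a player.
; AnyDamage records the shooter's PlayerState and expiry in Timers, while a repeat shot deactivates it if ShootToDeactivate is set.
; Authority Tick expires entries when ActiveDuration is positive, and OnReset clears a given player's entry.
; Activate and deactivate events notify the movers and swap the cube material only if that player is player controller 0.
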(event `self.ReceiveBeginPlay`)

(event `self.ReceiveActorBeginOverlap`
  (params (OtherActor :type "Actor Object Reference")))

(event `self.ReceiveAnyDamage`
  (params (Damage :type "Float (single-precision)") (DamageType :type "DamageType Object Reference") (InstigatedBy :type "Controller Object Reference") (DamageCauser :type "Actor Object Reference"))
  (bind _asutplayer_controller (cast `UTPlayerController` InstigatedBy))
  (bind _asbp_speed_player_state (cast `/Game/Speed/Blueprints/BP_SpeedPlayerState` (`Controller.PlayerState` _asutplayer_controller)))
  ;[1 1 1] Check if this player has already activated this trigger
  (set `self.bFound` false)
  (for _array_element (`self.Timers`)
    (if (== (`.PS_2_2E86B0824912377DC2C7B4979CA4A47A` (break `/Game/Speed/Blueprints/S_TriggerTime` _array_element)) _asbp_speed_player_state)
      (set `self.bFound` true)
      (break)))
  (if (`self.bFound`)
    (if (`self.ShootToDeactivate`)
      (`self.RemovePS` _asbp_speed_player_state))
    (else
      (`KismetArrayLibrary.Array_Add` (`self.Timers`) (make `/Game/Speed/Blueprints/S_TriggerTime` _asbp_speed_player_state (+ (`self.ActiveDuration`) (`KismetSystemLibrary.GetGameTimeInSeconds`))))
      (`self.OnActivate` _asbp_speed_player_state))))

(event `self.ReceiveTick`
  (params (DeltaSeconds :type "Float (single-precision)"))
  (bind _timers (`self.Timers`))
  (bind _i (`self.i`))
  (bind (_ps _endtime) (break `/Game/Speed/Blueprints/S_TriggerTime` (`KismetArrayLibrary.Array_Get` _timers (`self.i`))))
  (`/Engine/EditorBlueprintResources/ActorMacros.Switch Has Authority`
    (:`Authority`
      (if (> (`self.ActiveDuration`) 0.0)
        (bind _output_get (set `self.i` 0))
        (while (< _output_get (`KismetArrayLibrary.Array_Length` _timers))
          (if (> (`KismetSystemLibrary.GetGameTimeInSeconds`) _endtime)
            (`self.OnDeactivate` _ps)
            (`KismetArrayLibrary.Array_Remove` (`self.Timers`) _i)
            (else
              (set `self.i` (+ _i 1)))))))))

(event `OnDeactivate`
  (params (PS :type "/Game/Speed/Blueprints/BP_SpeedPlayerState Object Reference"))
  (bind _returnvalue (`GameplayStatics.GetPlayerController` 0))
  (for _array_element (`self.TriggerMover`)
    (`/Game/Speed/BP_SpeedMover.OnTriggered` _array_element PS false))
  (`/Engine/EditorBlueprintResources/StandardMacros.IsValid` _returnvalue
    (:`Is Valid`
      (bind _asbp_speed_player_state (cast `/Game/Speed/Blueprints/BP_SpeedPlayerState` (`Controller.PlayerState` _returnvalue)))
      (if (== _asbp_speed_player_state PS)
        (`PrimitiveComponent.SetMaterial` (`self.Cube`) 0 "/Game/Speed/Material/Switch/MI_SwitchOff.MI_SwitchOff")))))

(event `OnReset`
  (params (PS :type "/Game/Speed/Blueprints/BP_SpeedPlayerState Object Reference"))
  (`self.RemovePS` PS))

(event `OnActivate`
  (params (PS :type "/Game/Speed/Blueprints/BP_SpeedPlayerState Object Reference"))
  (bind _returnvalue (`GameplayStatics.GetPlayerController` 0))
  (for _array_element (`self.TriggerMover`)
    (`/Game/Speed/BP_SpeedMover.OnTriggered` _array_element PS true))
  (`/Engine/EditorBlueprintResources/StandardMacros.IsValid` _returnvalue
    (:`Is Valid`
      (bind _asbp_speed_player_state (cast `/Game/Speed/Blueprints/BP_SpeedPlayerState` (`Controller.PlayerState` _returnvalue)))
      (if (== _asbp_speed_player_state PS)
        (`PrimitiveComponent.SetMaterial` (`self.Cube`) 0 "/Game/Speed/Material/Switch/MI_SwitchOn.MI_SwitchOn")))))

(fn `RemovePS`
  (params (PS :type "/Game/Speed/Blueprints/BP_SpeedPlayerState Object Reference"))
  (bind _timers (`self.Timers`))
  (for (_array_element _array_index) _timers
    (bind _ps (break `/Game/Speed/Blueprints/S_TriggerTime` _array_element))
    (if (== _ps PS)
      (`self.OnDeactivate` _ps)
      (`KismetArrayLibrary.Array_Remove` _timers _array_index)
      (break))))

(fn `UserConstructionScript`)