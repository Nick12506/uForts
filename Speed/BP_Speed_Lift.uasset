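; BP_Speed_Lift is an Unreal Tournament lift that moves a mesh along a curve-driven timeline between its start and a grey transparent preview destination.
; Construction applies mesh, materials, destination and travel-time play rate; BeginPlay caches both endpoints on authority.
; Step-on, start, retrigger and encroach events are empty, their logic left unwired, leaving only LiftReverse driving the timeline.
; CreateSlave spawns a BP_Speed_Lift_Clone with copied settings, a given PlayerState and this lift as parent.
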(event `self.ReceiveBeginPlay`
  ;[1 1 1] On Begin Play- set up replicated lift positions
  (`/Engine/EditorBlueprintResources/ActorMacros.Switch Has Authority`
    (:`Authority`
      (set `self.Start Loc` (`SceneComponent.K2_GetComponentLocation` (`self.Mesh`)))
      (set `self.End Loc` (`SceneComponent.K2_GetComponentLocation` (`self.Top Preview`))))))

(event `self.AddBasedCharacter`
  (params (BasedCharacter :type "UTCharacter Object Reference"))
  ;[1 1 1] When someone steps on the lift
)

(event `LiftStart`
  ;[1 1 1] start lift if UTChars are based on it
)

(event `LiftReTrigger`
  ;[1 1 1] start lift if UTChars are based on it
)

(event `self.OnEncroachActor`
  (params (EncroachedActor :type "Actor Object Reference"))
  ;[1 1 1] lift encroached on UTChar
)

(event `LiftReverse`
  ;[1 1 1] wait at top time hit
  (`UTGameplayStatics.UTPlaySound` (`self.CloseStartSound`) self)
  (bind (_direction _0_1_lerp) (`Timeline|Lift Move` :!via `ReverseFromEnd`)
    (:`Update`
      ;[1 1 1] Move Lift
      (`self.MoveLiftTo` (`KismetMathLibrary.VLerp` (`self.Start Loc`) (`self.End Loc`) (`CurveFloat.GetFloatValue` (`self.Movement Curve`) _0_1_lerp))))
    (:`Finished`
      (`/Engine/EditorBlueprintResources/ActorMacros.Switch Has Authority`
        (:`Authority`
          (switch `TimelineComponent.ETimelineDirection` _direction
            (:`Forward`
              ;[1 1 1] lift is open
              (`UTGameplayStatics.UTPlaySound` (`self.OpenStopSound`) self)
              (`KismetSystemLibrary.K2_SetTimer` null "LiftReverse" (`self.Wait at top time`)))
            (:`Backward`
              ;[1 1 1] lift is closed
              (`UTGameplayStatics.UTPlaySound` (`self.CloseStopSound`) self)
              (set `self.bLiftIsMoving` false)
              (`KismetSystemLibrary.K2_SetTimer` null "LiftReTrigger" (`self.Retrigger Delay`)))))))))

(fn `CreateSlave`
  (params (PS :type "/Game/Speed/Blueprints/BP_SpeedPlayerState Object Reference"))
  (returns (Slave :type "/Game/Speed/Blueprints/I_Slave Interface"))
  (bind _overridematerial (`self.OverrideMaterial`))
  (bind _returnvalue (`|SpawnActorFromClass` "/Game/Speed/Blueprints/BP_Speed_Lift_Clone.BP_Speed_Lift_Clone_C" (`self.GetTransform`) true (`self.Mesh Scale`) (`self.Lift Destination`) (`self.Lift Mesh`) (`self.Lift Time`) (`self.Wait at top time`) (`self.Retrigger Delay`) (`self.Start Loc`) (`self.End Loc`) PS self))
  (`/Engine/EditorBlueprintResources/StandardMacros.IsValid` _overridematerial
    (:`Is Valid`
      (`PrimitiveComponent.SetMaterial` (`/Game/Speed/Blueprints/BP_Speed_Lift_Clone.Mesh` _returnvalue) 0 _overridematerial)
      (return _returnvalue))))

(fn `GetStops`
  (returns (ReturnValue :type "Array of Object.Vector Structure"))
  (return (`|MakeArray` (`SceneComponent.K2_GetComponentLocation` (`self.Mesh`)) (`SceneComponent.K2_GetComponentLocation` (`self.Top Preview`)))))

(fn `UserConstructionScript`
  (bind _mesh (`self.Mesh`))
  (bind _lift_mesh (`self.Lift Mesh`))
  (bind _top_preview (`self.Top Preview`))
  (`|ExecutionSequence`
    (:`then_0`
      (`SceneComponent.SetRelativeScale3D` (`self.Mesh`) (`self.Mesh Scale`))
      (`SceneComponent.SetRelativeScale3D` (`self.Top Preview`) (`self.Mesh Scale`))
      (`StaticMeshComponent.SetStaticMesh` _mesh _lift_mesh)
      (`self.SetEncroachComponent` _mesh)
      (`StaticMeshComponent.SetStaticMesh` _top_preview _lift_mesh)
      (`PrimitiveComponent.SetMaterial` _mesh 0 (`self.OverrideMaterial`))
      (`SceneComponent.K2_SetRelativeLocation` _top_preview (`self.Lift Destination`) false)
      (for _index (range (`PrimitiveComponent.GetNumMaterials` _top_preview))
        (`PrimitiveComponent.SetMaterial` _top_preview _index "/Game/RestrictedAssets/Effects/M_TransparentGrey.M_TransparentGrey")))
    (:`then_1`
      (`TimelineComponent.SetPlayRate` (`self.Lift Move`) (/ 1.0 (`self.Lift Time`))))))