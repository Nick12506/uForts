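; Player state for the Speed mode that tracks a player's run timing and manages per-player "slave" copies of master level actors.
; On BeginPlay it asks every I_Master actor to create a slave: always on the server, only for the local player's state on clients, using a retry timer until that state exists.
; Destruction notifies masters and slaves.
; RepNotifies record run start time and trigger the local HUD's score event.
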(event `self.ReceiveDestroyed`
  (`|ExecutionSequence`
    (:`then_0`
      (bind _outactors (`GameplayStatics.GetAllActorsWithInterface` "/Game/Speed/Blueprints/I_Master.I_Master_C"))
      (for _array_element _outactors
        (message `/Game/Speed/Blueprints/I_Master.OnDestroySlave` _array_element self)))
    (:`then_1`
      (bind _outactors_2 (`GameplayStatics.GetAllActorsWithInterface` "/Game/Speed/Blueprints/I_Slave.I_Slave_C"))
      (for _array_element_2 _outactors_2
        (message `/Game/Speed/Blueprints/I_Slave.DestroyByPlayerState` _array_element_2 self)))))

(event `self.ReceiveBeginPlay`
  (`parent.ReceiveBeginPlay`)
  (`/Engine/EditorBlueprintResources/ActorMacros.Switch Has Authority`
    (:`Authority`
      (bind _outactors (`GameplayStatics.GetAllActorsWithInterface` "/Game/Speed/Blueprints/I_Master.I_Master_C" :!label _label))
      (for _array_element _outactors
        (message `/Game/Speed/Blueprints/I_Master.CreateSlave` _array_element self)))
    (:`Remote`
      (`KismetSystemLibrary.K2_SetTimerDelegate` (delegate `InitLoop`) 0.2))))

(event `self.ReceiveActorBeginOverlap`
  (params (OtherActor :type "Actor Object Reference")))

(event `self.ReceiveTick`
  (params (DeltaSeconds :type "Float (single-precision)")))

(event `InitLoop`
  ;[1 1 1] seems to be some timing issues. loop until we have our local playerstate
  (bind _asbp_speed_player_state (cast `/Speed/Blueprints/BP_SpeedPlayerState` (`Controller.PlayerState` (`GameplayStatics.GetPlayerController` 0)))
    (:`then`
      (if (not (`self.init`))
        (set `self.init` true)
        (if (== _asbp_speed_player_state self)
          (goto _label))))
    (:`CastFailed`
      (`KismetSystemLibrary.K2_SetTimerDelegate` (delegate `InitLoop`) 0.2))))

(fn `OnRep_bIsRunning`
  (if (`self.bIsRunning`)
    (set `self.BeginTime` (`KismetSystemLibrary.GetGameTimeInSeconds`))))

(fn `OnRep_LastTime`
  (bind _returnvalue (`GameplayStatics.GetPlayerController` 0))
  (if (not (`KismetSystemLibrary.IsDedicatedServer`))
    (bind _asbp_speed_player_state (cast `/Speed/Blueprints/BP_SpeedPlayerState` (`Controller.PlayerState` _returnvalue)))
    (if (== _asbp_speed_player_state self)
      (bind _asbp_speed_hud (cast `/Game/Speed/Blueprints/BP_SpeedHUD` (`PlayerController.GetHUD` _returnvalue)))
      (`/Game/Speed/Blueprints/BP_SpeedHUD.OnScore` _asbp_speed_hud))))

(fn `UserConstructionScript`)