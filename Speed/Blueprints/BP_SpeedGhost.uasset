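; Speed ghost character that replays a recorded run from its GhostFrames array.
; Each tick it applies every frame whose timestamp has passed since BeginPlay, setting location, yaw, movement velocity and BP_GhostController's control rotation.
; Crouch state is read after the index increments, so it comes from the following frame.
; The ghost destroys itself once the frames run out.
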(event `self.ReceiveBeginPlay`
  (`parent.ReceiveBeginPlay`)
  (set `self.StartTime` (`KismetSystemLibrary.GetGameTimeInSeconds`)))

(event `self.ReceiveActorBeginOverlap`
  (params (OtherActor :type "Actor Object Reference")))

(event `self.ReceiveTick`
  (params (DeltaSeconds :type "Float (single-precision)"))
  (bind _ghostframes (`self.GhostFrames`))
  (bind (_time _location _rotation _controlrotation _velocity _crouch) (break `/Game/Speed/Blueprints/S_GhostFrame` (`KismetArrayLibrary.Array_Get` _ghostframes (`self.CurrentFrame`))))
  (bind _returnvalue (< (`self.CurrentFrame`) (`KismetArrayLibrary.Array_Length` _ghostframes)))
  (`parent.ReceiveTick` DeltaSeconds)
  (if _returnvalue
    (while (and (> (- (`KismetSystemLibrary.GetGameTimeInSeconds`) (`self.StartTime`)) _time) _returnvalue)
      (`self.K2_SetActorLocationAndRotation` _location (`KismetMathLibrary.MakeRot` 0.0 (.yaw _controlrotation)))
      (bind _asbp_ghost_controller (cast `/Game/Speed/Blueprints/BP_GhostController` (`self.GetController`))
        (:`then`
          (`Controller.SetControlRotation` _asbp_ghost_controller _controlrotation))
        (:`CastFailed`
          _))
      (set `MovementComponent.Velocity` _velocity (`self.UTCharacterMovement`))
      (set `self.CurrentFrame` (+ (`self.CurrentFrame`) 1))
      (if _crouch
        (`self.Crouch`)
        (else
          (`self.UnCrouch`))))
    (else
      (`self.K2_DestroyActor`))))

(fn `UserConstructionScript`
  (`parent.UserConstructionScript`))