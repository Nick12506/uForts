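; Helper function library for the Speed content, providing time formatting and a chat shortcut for Unreal Tournament.
; FormatTime turns seconds into a minutes, seconds and milliseconds text with zero padding, adding a leading minus for negative values.
; TimSay casts the first player controller to UTPlayerController and runs a "say" console command on it, appending the given string directly without a separating space.
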(fn `FormatTime`
  (params (Seconds :type "Float (double-precision)" :default 0.0))
  (returns (Out :type Text))
  (bind _returnvalue (`KismetMathLibrary.FromSeconds` (`KismetMathLibrary.Abs` Seconds)))
  (return (`|FormatText` (select `bool` (< Seconds 0.0) :`false` "{0} : {1} . {2}" :`true` "- {0} : {1} . {2}") (`KismetTextLibrary.Conv_IntToText` (`KismetMathLibrary.FFloor` (`KismetMathLibrary.GetTotalMinutes` _returnvalue))) (`KismetTextLibrary.Conv_IntToText` (`KismetMathLibrary.GetSeconds` _returnvalue) true 2 2) (`KismetTextLibrary.Conv_IntToText` (`KismetMathLibrary.GetMilliseconds` _returnvalue) true 3 3))))

(fn `TimSay`
  (params (Context :type "Object Object Reference") (Say :type String))
  (bind _asutplayer_controller (cast `UTPlayerController` (`GameplayStatics.GetPlayerController` Context)))
  (`KismetSystemLibrary.ExecuteConsoleCommand` _asutplayer_controller (`KismetStringLibrary.Concat_StrStr` "say " Say)))