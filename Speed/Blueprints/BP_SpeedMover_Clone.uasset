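; Per-player clone of a parent mover: a lift that only the character with the matching PlayerState collides with.
; On BeginPlay the authority copies start and end points from ParentMover; without a parent the clone destroys itself.
; A trigger counter, with optional modulus and threshold, plays or reverses a curve-eased timeline driving MoveLiftTo.
; Mutual move-ignores filter out other players, and the clone is destroyed by PlayerState.
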(event `self.UpdateCollisionIgnores`
  (params (Character :type "/Game/Speed/Blueprints/BP_SpeedCharacter Object Reference"))
  (`self.IgnoreOtherPlayers`))

(event `self.DestroyByPlayerState`
  (params (PS :type "/Game/Speed/Blueprints/BP_SpeedPlayerState Object Reference"))
  (bind _playerstate (`self.PlayerState`))
  (if (or (== PS _playerstate) (not (`KismetSystemLibrary.IsValid` _playerstate)))
    (`self.K2_DestroyActor`)))

(event `self.ReceiveBeginPlay`
  (bind _parentmover (`self.ParentMover`))
  (`/Engine/EditorBlueprintResources/StandardMacros.IsValid` _parentmover
    (:`Is Valid`
      (`self.IgnoreOtherPlayers`)
      ;[1 1 1] On Begin Play- set up replicated lift positions
      (`/Engine/EditorBlueprintResources/ActorMacros.Switch Has Authority`
        (:`Authority`
          (set `self.Start Loc` (`SceneComponent.K2_GetComponentLocation` (`/Game/Speed/BP_SpeedMover.Mesh` _parentmover)))
          (set `self.End Loc` (`SceneComponent.K2_GetComponentLocation` (`/Game/Speed/BP_SpeedMover.Top Preview` _parentmover))))))
    (:`Is Not Valid`
      (`self.K2_DestroyActor`))))

(event `OnTriggered`
  (params (Activate :type Boolean :default false))
  (bind _triggermodulus (`self.TriggerModulus`))
  (bind _output_get (set `self.TriggerCount` (+ (select `bool` Activate :`false` -1 :`true` 1) (`self.TriggerCount`))))
  (if (>= (select `bool` (> _triggermodulus 0) :`false` _output_get :`true` (mod _output_get _triggermodulus)) (`self.MinTrigger`))
    ;[1 1 1] start lift if UTChars are based on it
    (`UTGameplayStatics.UTPlaySound` (`self.OpenStartSound`) self :!label _label)
    (bind (_direction _0_1_lerp) (`Timeline|Lift Move` :!label _label_2)
      (:`Update`
        ;[1 1 1] Move Lift
        (`self.MoveLiftTo` (`KismetMathLibrary.VLerp` (`self.Start Loc`) (`self.End Loc`) (`CurveFloat.GetFloatValue` (`self.Movement Curve`) _0_1_lerp))))
      (:`Finished`
        (`/Engine/EditorBlueprintResources/ActorMacros.Switch Has Authority`
          (:`Authority`
            (switch `TimelineComponent.ETimelineDirection` _direction
              (:`Forward`
                ;[1 1 1] lift is open
                (`UTGameplayStatics.UTPlaySound` (`self.OpenStopSound`) self))
              (:`Backward`
                ;[1 1 1] lift is closed
                (`UTGameplayStatics.UTPlaySound` (`self.CloseStopSound`) self)
                (set `self.bLiftIsMoving` false)))))))
    (else
      ;[1 1 1] wait at top time hit
      (`UTGameplayStatics.UTPlaySound` (`self.CloseStartSound`) self :!label _label_3)
      (goto _label_2 :!via `Reverse`))))

(event `LiftStart`
  ;[1 1 1] start lift if UTChars are based on it
  (bind _returnvalue (`self.HasBasedCharacters`))
  (if _returnvalue
    (goto _label)
    (else
      (set `self.bLiftIsMoving` false))))

(event `LiftReverse`
  ;[1 1 1] wait at top time hit
  (goto _label_3))

(fn `GetStops`
  (returns (ReturnValue :type "Array of Object.Vector Structure"))
  (return (`|MakeArray` (`SceneComponent.K2_GetComponentLocation` (`self.Mesh`)) (`SceneComponent.K2_GetComponentLocation` (`self.Top Preview`)))))

(fn `IgnoreOtherPlayers`
  (bind _mesh (`self.Mesh`))
  (`PrimitiveComponent.ClearMoveIgnoreActors` _mesh)
  (`PrimitiveComponent.ClearMoveIgnoreActors`)
  (bind _outactors (`GameplayStatics.GetAllActorsOfClass` "/Game/Speed/Blueprints/BP_SpeedCharacter.BP_SpeedCharacter_C"))
  (for _array_element _outactors
    (bind _returnvalue (or (!= (`Pawn.PlayerState` _array_element) (`self.PlayerState`)) (not (`KismetSystemLibrary.IsValid` (`self.PlayerState`)))))
    (`PrimitiveComponent.IgnoreActorWhenMoving` _mesh _array_element _returnvalue)
    (`PrimitiveComponent.IgnoreActorWhenMoving` _array_element _returnvalue)
    (`PrimitiveComponent.IgnoreActorWhenMoving` _array_element self _returnvalue)))

(fn `UserConstructionScript`
  (bind _mesh (`self.Mesh`))
  (bind _lift_mesh (`self.Lift Mesh`))
  (bind _top_preview (`self.Top Preview`))
  (`|ExecutionSequence`
    (:`then_0`
      (`SceneComponent.SetRelativeScale3D` (`self.Mesh`) (`self.Mesh Scale`))
      (`SceneComponent.SetRelativeScale3D` (`self.Top Preview`) (`self.Mesh Scale`))
      (`StaticMeshComponent.SetStaticMesh` _mesh _lift_mesh)
      (`self.SetEncroachComponent` _mesh)
      (`StaticMeshComponent.SetStaticMesh` _top_preview _lift_mesh)
      (`PrimitiveComponent.SetMaterial` _mesh 0 (`self.OverrideMaterial`))
      (`SceneComponent.K2_SetRelativeLocation` _top_preview (`self.Lift Destination`) false)
      (for _index (range (`PrimitiveComponent.GetNumMaterials` _top_preview))
        (`PrimitiveComponent.SetMaterial` _top_preview _index "/Game/RestrictedAssets/Effects/M_TransparentGrey.M_TransparentGrey")))
    (:`then_1`
      (`TimelineComponent.SetPlayRate` (`self.Lift Move`) (/ 1.0 (`self.Lift Time`))))))