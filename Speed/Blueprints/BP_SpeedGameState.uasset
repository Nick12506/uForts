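; Game state for the Speed mode that tracks each player's best run and the map's all-time best time.
; On the server, PlayerFinished updates the player state's personal best and saves any new map record to a BP_SpeedSave slot, which BeginPlay reloads.
; The slot name comes from the map's BP_SpeedInfo actor, and persistence is skipped without one.
; OnNewScore is an empty hook for ServerStatsPlugin, called on every finish.
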(event `self.ReceiveBeginPlay`
  (bind _slotname (`self.GetSaveName`))
  (`/Engine/EditorBlueprintResources/ActorMacros.Switch Has Authority`
    (:`Authority`
      (if (not (`KismetStringLibrary.EqualEqual_StrStr` _slotname "NOSAVE"))
        (bind _returnvalue (`GameplayStatics.LoadGameFromSlot` _slotname))
        (bind _asbp_speed_save (cast `/Game/Speed/Blueprints/BP_SpeedSave` _returnvalue))
        (set `self.BestTime` (`/Game/Speed/Blueprints/BP_SpeedSave.HiScore` _asbp_speed_save))))))

(event `self.ReceiveActorBeginOverlap`
  (params (OtherActor :type "Actor Object Reference")))

(event `self.ReceiveTick`
  (params (DeltaSeconds :type "Float (single-precision)")))

(fn `GetSaveName`
  (returns (SlotName :type String))
  (bind _outactors (`GameplayStatics.GetAllActorsOfClass` "/Game/Speed/BP_SpeedInfo.BP_SpeedInfo_C"))
  (return (select `bool` (> (`KismetArrayLibrary.Array_Length` _outactors) 0) :`false` "NOSAVE" :`true` (`KismetStringLibrary.Concat_StrStr` "SPEEDSAVE-" (`/Game/Speed/BP_SpeedInfo.SaveMapName` (`KismetArrayLibrary.Array_Get` _outactors))))))

(fn `OnNewScore`
  (params (NewScore :type "/Game/Speed/Blueprints/S_HiScore Structure")))

(fn `OnRep_LeaderBoard`)

(fn `PlayerFinished`
  (params (Score :type "/Game/Speed/Blueprints/S_HiScore Structure") (Player :type "/Game/Speed/Blueprints/BP_SpeedCharacter Object Reference"))
  (bind _time (break `/Game/Speed/Blueprints/S_HiScore` Score))
  (bind _slotname (`self.GetSaveName`))
  (bind _time_2 (break `/Game/Speed/Blueprints/S_HiScore` (`self.BestTime`)))
  (`/Engine/EditorBlueprintResources/ActorMacros.Switch Has Authority`
    (:`Authority`
      (`self.OnNewScore` Score) ; This gets hooked by the ServerStatsPlugin
      (`|ExecutionSequence`
        (:`then_0`
          (bind _asbp_speed_player_state (cast `/Game/Speed/Blueprints/BP_SpeedPlayerState` (`Pawn.PlayerState` Player)))
          (bind _mybest (`/Game/Speed/Blueprints/BP_SpeedPlayerState.MyBest` _asbp_speed_player_state))
          (if (or (== _mybest 0.0) (> _mybest _time))
            (set `/Game/Speed/Blueprints/BP_SpeedPlayerState.MyBest` _time _asbp_speed_player_state)))
        (:`then_1`
          (if (or (< _time _time_2) (== _time_2 0.0))
            (bind _output_get (set `self.BestTime` Score))
            (bind _returnvalue (`GameplayStatics.CreateSaveGameObject` "/Game/Speed/Blueprints/BP_SpeedSave.BP_SpeedSave_C"))
            (bind _asbp_speed_save (cast `/Game/Speed/Blueprints/BP_SpeedSave` _returnvalue))
            (set `/Game/Speed/Blueprints/BP_SpeedSave.HiScore` _output_get _asbp_speed_save)
            (if (not (`KismetStringLibrary.EqualEqual_StrStr` _slotname "NOSAVE"))
              (`GameplayStatics.SaveGameToSlot` _asbp_speed_save _slotname))))))))

(fn `UserConstructionScript`)